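; BP_P_Ingredient is an ingredient pickup that shows an on-screen widget when it is processed.
; BeginPlay creates an IngredientWidget and hands it a reference to the actor.
; OnBeingProcessed runs the parent logic, then adds the widget to the viewport if it is not already there.
; Tick projects the actor's location to screen space, keeping the widget just below that point.
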(event EventBeginPlay
  (bind _returnvalue (UserInterface|CreateWidget "/Game/Blueprint/HUD/IngredientWidget.IngredientWidget_C"))
  (bind _output_get (Variables|Default|SetCurrentWidget _returnvalue))
  (bind _asingredient_widget (Utilities|Casting|CastToIngredientWidget _output_get))
  (Variables|/Game/Blueprint/HUD/IngredientWidget.IngredientWidget_C|SetIngredientRef _asingredient_widget self))

(event EventTick
  (params (DeltaSeconds :type Float%20%28single-precision%29))
  (if (Utilities|IsValid (Variables|Default|GetCurrentWidget))
    (Class|UserWidget|SetPositioninViewport (Variables|Default|GetCurrentWidget) (- (.ScreenLocation (Class|PlayerController|ProjectWorldLocationtoScreen (Game|GetPlayerController 0) (Transformation|GetActorLocation) false)) "(X=0.000000,Y=-15.000000)") true)))

(event EventOnBeingProcessed
  (|CallParentFunction)
  (if (not (UserInterface|Viewport|IsinViewport (Variables|Default|GetCurrentWidget)))
    (UserInterface|Viewport|AddtoViewport (Variables|Default|GetCurrentWidget) 0)))

(fn ConstructionScript)