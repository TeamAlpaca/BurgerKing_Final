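; BP_P_Food is a food pickup Blueprint that shows an on-screen widget once the food starts being overcooked.
; On that event it calls the parent, creates a FoodWidget on first use with a reference back to itself, and adds it to the viewport.
; Each Tick projects the actor's world location to screen space and moves the widget there, so it follows the food.
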(event EventTick
  (params (DeltaSeconds :type Float%20%28single-precision%29))
  (if (Utilities|IsValid (Variables|Default|GetCurrentWidget))
    (Class|UserWidget|SetPositioninViewport (Variables|Default|GetCurrentWidget) (.ScreenLocation (Class|PlayerController|ProjectWorldLocationtoScreen (Game|GetPlayerController 0) (Transformation|GetActorLocation) false)) true)))

(event EventOnStartBeingOvercooked
  (|CallParentFunction)
  (if (Utilities|IsValid (Variables|Default|GetCurrentWidget))
    _
    (else
      (bind _returnvalue (UserInterface|CreateWidget "/Game/Blueprint/HUD/FoodWidget.FoodWidget_C"))
      (bind _output_get (Variables|Default|SetCurrentWidget _returnvalue))
      (bind _asfood_widget (Utilities|Casting|CastToFoodWidget _output_get))
      (Variables|/Game/Blueprint/HUD/FoodWidget.FoodWidget_C|SetFoodRef _asfood_widget self)))
  (if (not (UserInterface|Viewport|IsinViewport (Variables|Default|GetCurrentWidget)))
    (UserInterface|Viewport|AddtoViewport (Variables|Default|GetCurrentWidget) 0)))

(fn ConstructionScript)