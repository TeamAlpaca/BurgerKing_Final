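; Plate pickup Blueprint that shows an on-screen widget when the plate is being cleaned.
; OnBeingCleaned calls the parent event, lazily creates the PlateWidget with a reference back to the plate, and adds it to the viewport if absent.
; Tick projects the plate's world location to screen space each frame so the widget follows it.
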(event EventBeginPlay)

(event EventTick
  (params (DeltaSeconds :type Float%20%28single-precision%29))
  ;[1 1 1] Update Widget Position
  (if (Utilities|IsValid (Variables|Default|GetCurrentWidget))
    (Class|UserWidget|SetPositioninViewport (Variables|Default|GetCurrentWidget) (.ScreenLocation (Class|PlayerController|ProjectWorldLocationtoScreen (Game|GetPlayerController 0) (Transformation|GetActorLocation) false)) true)))

(event EventOnBeingCleaned
  ;[1 1 1] Add Wiget
  (|CallParentFunction)
  (Utilities|IsValid (Variables|Default|GetCurrentWidget)
    (:Is%20Valid
      _)
    (:Is%20Not%20Valid
      (bind _returnvalue (UserInterface|CreateWidget "/Game/Blueprint/HUD/PlateWidget.PlateWidget_C"))
      (bind _output_get (Variables|Default|SetCurrentWidget _returnvalue))
      (bind _asplate_widget (Utilities|Casting|CastToPlateWidget _output_get))
      (Variables|/Game/Blueprint/HUD/PlateWidget.PlateWidget_C|SetPlateRef _asplate_widget self)))
  (if (not (UserInterface|Viewport|IsinViewport (Variables|Default|GetCurrentWidget)))
    (UserInterface|Viewport|AddtoViewport (Variables|Default|GetCurrentWidget) 0)))

(fn ConstructionScript)